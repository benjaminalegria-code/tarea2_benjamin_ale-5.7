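; BP_enemy is an enemy actor that takes hits, shows its health on a widget component and dies when its health runs out.
; The RecibirGolpe (receive hit) event subtracts a fixed amount of HP, prints it and updates the WBP_EnemyHP progress bar.
; At zero or below it plays a 2D death sound and destroys the actor, but this check runs only if the widget cast succeeds.
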(event `RecibirGolpe`
  (bind _output_get (set `self.HP` (- (`self.HP`) 20.0)))
  (`KismetSystemLibrary.PrintString` (`KismetStringLibrary.Conv_DoubleToString` _output_get))
  (bind _aswbp_enemy_hp (cast `/Game/player/WB/WBP_EnemyHP` (`WidgetComponent.GetUserWidgetObject` (`self.HPbar`))))
  (`ProgressBar.SetPercent` (`/Game/player/WB/WBP_EnemyHP.PB_HP` _aswbp_enemy_hp) (/ (`self.HP`) 100.0))
  (if (<= _output_get 0.0)
    (`GameplayStatics.PlaySound2D` "/Game/Roblox_Death_Sound__Oof__-_Sound_Effect__HD_.Roblox_Death_Sound__Oof__-_Sound_Effect__HD_" 1.0 1.0 0.0 null null)
    (`self.K2_DestroyActor`)))

(fn `UserConstructionScript`)