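; Player character Blueprint with Enhanced Input movement, camera look, jump, run and melee combat.
; Interact prioritizes the nearby NPC, falling back to the nearby chest.
; Attack drives a three-step montage combo through an index and a CanChain gate, which is never opened here, resetting when a montage completes.
; DetectarGolpe, not called within this graph, sphere-traces ahead and notifies any BP_enemy it hits.
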(event `EnhancedInput|/Game/blueprints/IA_interact`
  (params (ActionValue :type Boolean) (ElapsedSeconds :type "Float (double-precision)") (TriggeredSeconds :type "Float (double-precision)") (InputAction :type "InputAction Object Reference" :default "/Game/blueprints/IA_interact.IA_interact"))
  (bind _npccercano (`self.NPCcercano`))
  (bind _cofrecercano (`self.CofreCercano`))
  (:`Started`
    (`/Engine/EditorBlueprintResources/StandardMacros.IsValid` _npccercano
      (:`Is Valid`
        (`/Game/player/BP_npc.InteractuarNpc` _npccercano))
      (:`Is Not Valid`
        (`/Engine/EditorBlueprintResources/StandardMacros.IsValid` _cofrecercano
          (:`Is Valid`
            (`/Game/player/BP_cofre.IntentarAbrir` _cofrecercano)))))))

(event `EnhancedInput|/Game/blueprints/IA_jump`
  (params (ActionValue :type Boolean) (ElapsedSeconds :type "Float (double-precision)") (TriggeredSeconds :type "Float (double-precision)") (InputAction :type "InputAction Object Reference" :default "/Game/blueprints/IA_jump.IA_jump"))
  (:`Triggered`
    (`self.Jump`)))

(event `self.ReceiveBeginPlay`
  (`EnhancedInputSubsystemInterface.AddMappingContext` (pcsubsystem `EnhancedInputLocalPlayerSubsystem` (`GameplayStatics.GetPlayerController` 0)) "/Game/blueprints/IMC_player.IMC_player" 0 (struct)))

(event `EnhancedInput|/Game/blueprints/IA_Run`
  (params (ActionValue :type Boolean) (ElapsedSeconds :type "Float (double-precision)") (TriggeredSeconds :type "Float (double-precision)") (InputAction :type "InputAction Object Reference" :default "/Game/blueprints/IA_Run.IA_Run"))
  (:`Started`
    (set `CharacterMovementComponent.MaxWalkSpeed` 600.0 (`self.CharacterMovement`)))
  (:`Completed`
    (set `CharacterMovementComponent.MaxWalkSpeed` 300.0 (`self.CharacterMovement`))))

(event `EnhancedInput|/Game/blueprints/IA_cam`
  (params (ActionValue :type "Vector2D Structure") (ElapsedSeconds :type "Float (double-precision)") (TriggeredSeconds :type "Float (double-precision)") (InputAction :type "InputAction Object Reference" :default "/Game/blueprints/IA_cam.IA_cam"))
  (:`Triggered`
    (`self.AddControllerYawInput` ActionValue_X)
    (`self.AddControllerPitchInput` ActionValue_Y)))

(event `EnhancedInput|/Game/blueprints/IA_move`
  (params (ActionValue :type "Vector2D Structure") (ElapsedSeconds :type "Float (double-precision)") (TriggeredSeconds :type "Float (double-precision)") (InputAction :type "InputAction Object Reference" :default "/Game/blueprints/IA_move.IA_move"))
  (bind (_returnvalue_roll _returnvalue_pitch _returnvalue_yaw) (`KismetMathLibrary.BreakRotator` (`self.GetControlRotation`)))
  (bind (_returnvalue_roll_2 _returnvalue_pitch_2 _returnvalue_yaw_2) (`KismetMathLibrary.BreakRotator` (`self.GetControlRotation`)))
  (:`Triggered`
    (`self.AddMovementInput` (`KismetMathLibrary.GetForwardVector` (`KismetMathLibrary.MakeRotator` 0.0 0.0 _returnvalue_yaw_2)) ActionValue_X)
    (`self.AddMovementInput` (`KismetMathLibrary.GetRightVector` (`KismetMathLibrary.MakeRotator` 0.0 0.0 _returnvalue_yaw)) ActionValue_Y)))

(event `EnhancedInput|/Game/blueprints/IA_attack`
  (params (ActionValue :type Boolean) (ElapsedSeconds :type "Float (double-precision)") (TriggeredSeconds :type "Float (double-precision)") (InputAction :type "InputAction Object Reference" :default "/Game/blueprints/IA_attack.IA_attack"))
  (:`Started`
    (if (`self.blsAttacking`)
      (if (`self.bCanChain`)
        (if (< (`self.ComboIndex`) 3)
          (`/Engine/EditorBlueprintResources/StandardMacros.IncrementInt` (`self.ComboIndex`)
            (:`  `
              (set `self.bCanChain` false)
              (`self.ExcuteCurrentAttack`)))))
      (else
        (set `self.ComboIndex` 1)
        (set `self.blsAttacking` true)
        (set `self.bCanChain` false)
        (`self.ExcuteCurrentAttack`)))))

(event `ExcuteCurrentAttack`
  (bind _mesh (`self.Mesh`))
  (switch `int` (`self.ComboIndex`)
    (:`1`
      (`|PlayMontage` _mesh "/Game/animation/montage_attack1.montage_attack1"
        (:`OnCompleted`
          (`KismetSystemLibrary.PrintString` "TERMINADO")
          (set `self.ComboIndex` 0)
          (set `self.blsAttacking` false)
          (set `self.bCanChain` false))
        (:`OnInterrupted`
          (`KismetSystemLibrary.PrintString` "INTERRUMPIDO"))))
    (:`2`
      (`|PlayMontage` _mesh "/Game/animation/montage_attack2.montage_attack2"
        (:`OnCompleted`
          (set `self.ComboIndex` 0)
          (set `self.blsAttacking` false)
          (set `self.bCanChain` false))))
    (:`3`
      (`|PlayMontage` _mesh "/Game/animation/montage_attack3.montage_attack3"
        (:`OnCompleted`
          (set `self.ComboIndex` 0)
          (set `self.blsAttacking` false)
          (set `self.bCanChain` false))))))

(event `DetectarGolpe`
  (bind (_outhit _returnvalue) (`KismetSystemLibrary.SphereTraceSingle` :`Start` (`self.K2_GetActorLocation`) :`End` (+ (* (`self.GetActorForwardVector`) (150.0 150.0 150.0)) (`self.K2_GetActorLocation`)) :`Radius` 75.0 :`TraceChannel` "TraceTypeQuery1" :`DrawDebugType` "ForDuration"))
  (if _returnvalue
    (bind _asbp_enemy (cast `/Game/player/BP_enemy` (`.HitActor` (`GameplayStatics.BreakHitResult` _outhit))))
    (`/Game/player/BP_enemy.RecibirGolpe` _asbp_enemy)))

(fn `UserConstructionScript`)