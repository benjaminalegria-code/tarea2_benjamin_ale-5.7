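; BP_npc is a talkable NPC that shows its lines of dialogue one at a time in a WBP_Dialogo widget.
; Its ZonaDialogo overlap volume registers the NPC as the player's NPCcercano on entry and clears it on exit.
; Each InteractuarNpc call creates the widget or advances through the Dialogo array by index, then removes the widget and resets after the last line.
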(event `self.ZonaDialogo.OnComponentBeginOverlap`
  (params (OverlappedComponent :type "PrimitiveComponent Object Reference") (OtherActor :type "Actor Object Reference") (OtherComp :type "PrimitiveComponent Object Reference") (OtherBodyIndex :type Integer) (bFromSweep :type Boolean) (SweepResult :type "HitResult Structure (by ref)"))
  (bind _asbp_player (cast `/Game/player/BP_player` OtherActor))
  (set `/Game/player/BP_player.NPCcercano` self _asbp_player))

(event `self.ZonaDialogo.OnComponentEndOverlap`
  (params (OverlappedComponent :type "PrimitiveComponent Object Reference") (OtherActor :type "Actor Object Reference") (OtherComp :type "PrimitiveComponent Object Reference") (OtherBodyIndex :type Integer))
  (bind _asbp_player (cast `/Game/player/BP_player` OtherActor))
  (set `/Game/player/BP_player.NPCcercano` null _asbp_player))

(event `InteractuarNpc`
  (`/Engine/EditorBlueprintResources/StandardMacros.IsValid` (`self.WidgetDialogo`)
    (:`Is Valid`
      (if (< (`self.IndiceDialogo`) (`KismetArrayLibrary.Array_Length` (`self.Dialogo`)))
        (`/Game/player/WB/WBP_Dialogo.ActualizarDialogo` (`self.WidgetDialogo`) (`|GetArrayItem` (`self.Dialogo`) (`self.IndiceDialogo`)))
        (set `self.IndiceDialogo` (+ (`self.IndiceDialogo`) 1))
        (else
          (`Widget.RemoveFromParent` (`self.WidgetDialogo`))
          (set `self.WidgetDialogo` null)
          (set `self.IndiceDialogo` 0))))
    (:`Is Not Valid`
      (bind _returnvalue (`|CreateWidget` "/Game/player/WB/WBP_Dialogo.WBP_Dialogo_C" (`GameplayStatics.GetPlayerController` 0)))
      (bind _output_get (set `self.WidgetDialogo` _returnvalue))
      (`UserWidget.AddToViewport` _output_get 0)
      (`/Game/player/WB/WBP_Dialogo.ActualizarDialogo` (`self.WidgetDialogo`) (`|GetArrayItem` (`self.Dialogo`)))
      (set `self.IndiceDialogo` 1))))

(fn `UserConstructionScript`)