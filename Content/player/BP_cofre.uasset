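; Chest actor that opens only when the player holds a key, revealing a final objective.
; Its overlap zone sets and clears itself as the player's nearby chest reference (CofreCercano).
; IntentarAbrir checks TieneLlave on the player, then marks the chest open once, swaps its material, plays a sound and enables the referenced objective's visibility and collision.
; Without a key it prints a debug message.
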(event `self.ZonaCofre.OnComponentBeginOverlap`
  (params (OverlappedComponent :type "PrimitiveComponent Object Reference") (OtherActor :type "Actor Object Reference") (OtherComp :type "PrimitiveComponent Object Reference") (OtherBodyIndex :type Integer) (bFromSweep :type Boolean) (SweepResult :type "HitResult Structure (by ref)"))
  (bind _asbp_player (cast `/Game/player/BP_player` OtherActor))
  (set `/Game/player/BP_player.CofreCercano` self _asbp_player))

(event `IntentarAbrir`
  (if (not (`self.bAbierto`))
    (bind _asbp_player (cast `/Game/player/BP_player` (`GameplayStatics.GetPlayerCharacter` 0)))
    (if (`/Game/player/BP_player.TieneLlave` _asbp_player)
      (set `self.bAbierto` true)
      (`PrimitiveComponent.SetMaterial` (`self.cofre`) 0 "/Game/material/M_CofreAbierto.M_CofreAbierto")
      (`GameplayStatics.PlaySoundAtLocation` "/Game/Open_Chest__Minecraft____Sound_Effect.Open_Chest__Minecraft____Sound_Effect" (`self.K2_GetActorLocation`) (struct) 1.0 1.0 0.0 null null null null)
      (`/Engine/EditorBlueprintResources/StandardMacros.IsValid` (`self.ObjetiFinalRef`)
        (:`Is Valid`
          (`self.SetActorHiddenInGame` (`self.ObjetiFinalRef`) false)
          (`self.SetActorEnableCollision` (`self.ObjetiFinalRef`) true)))
      (else
        (`KismetSystemLibrary.PrintString` "no tengo llave")))))

(event `self.ZonaCofre.OnComponentEndOverlap`
  (params (OverlappedComponent :type "PrimitiveComponent Object Reference") (OtherActor :type "Actor Object Reference") (OtherComp :type "PrimitiveComponent Object Reference") (OtherBodyIndex :type Integer))
  (bind _asbp_player (cast `/Game/player/BP_player` OtherActor))
  (set `/Game/player/BP_player.CofreCercano` null _asbp_player))

(fn `UserConstructionScript`)